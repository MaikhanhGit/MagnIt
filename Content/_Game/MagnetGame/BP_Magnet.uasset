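; Player-controlled magnet pawn that moves, yaws and handles red and black tagged objects.
; Flip-flopped timelines rotate its Cube vertically and horizontally, with the vertical state gating horizontal turning and collection.
; Per-color push colliders launch tagged overlaps forward with physics force, while destination colliders record collected tins.
; BPCMagnet activates on BeginPlay; ReleaseRedTin frees the held red tin and re-enables vertical turning, while ReleaseBlackTin is empty.
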(event OnComponentBeginOverlap(BlackDestCol)
  (params (OverlappedComponent :type Primitive%20Component%20Object%20Reference) (OtherActor :type Actor%20Object%20Reference) (OtherComp :type Primitive%20Component%20Object%20Reference) (OtherBodyIndex :type Integer) (bFromSweep :type Boolean) (SweepResult :type Hit%20Result%20Structure%20%28by%20ref%29))
  ;[0.15 0.15 0.15 0.5] Check If Holding Anything
  (if (Actor|ActorHasTag OtherActor "MagBlack")
    (Variables|Default|SetCollectedBlackTin OtherActor)
    (Variables|Default|SetIsBlackFull? true)
    (Variables|Default|SetisBlackCollected? true)))

(event OnComponentEndOverlap(RedDestCol)
  (params (OverlappedComponent :type Primitive%20Component%20Object%20Reference) (OtherActor :type Actor%20Object%20Reference) (OtherComp :type Primitive%20Component%20Object%20Reference) (OtherBodyIndex :type Integer))
  ;[0.15 0.15 0.15 0.5] NOT USED
)

(event OnComponentBeginOverlap(RedDestCol)
  (params (OverlappedComponent :type Primitive%20Component%20Object%20Reference) (OtherActor :type Actor%20Object%20Reference) (OtherComp :type Primitive%20Component%20Object%20Reference) (OtherBodyIndex :type Integer) (bFromSweep :type Boolean) (SweepResult :type Hit%20Result%20Structure%20%28by%20ref%29))
  ;[0.15 0.15 0.15 0.5] Check If Holding Anything
  (if (Actor|ActorHasTag OtherActor "MagRed")
    (Variables|Default|SetCollectedRedTin OtherActor)
    (Variables|Default|SetIsRedFull? true)
    (Variables|Default|SetisRedCollected? true)))

(event OnComponentEndOverlap(BlackDestCol)
  (params (OverlappedComponent :type Primitive%20Component%20Object%20Reference) (OtherActor :type Actor%20Object%20Reference) (OtherComp :type Primitive%20Component%20Object%20Reference) (OtherBodyIndex :type Integer))
  ;[0.15 0.15 0.15 0.5] NOT USED
)

(event OnComponentBeginOverlap(BlackPushCol)
  (params (OverlappedComponent :type Primitive%20Component%20Object%20Reference) (OtherActor :type Actor%20Object%20Reference) (OtherComp :type Primitive%20Component%20Object%20Reference) (OtherBodyIndex :type Integer) (bFromSweep :type Boolean) (SweepResult :type Hit%20Result%20Structure%20%28by%20ref%29))
  ;[0.15 0.15 0.15 0.5] Push BLAK
  (if (Actor|ActorHasTag OtherActor (Variables|Default|GetTagBlack))
    (Variables|Default|SetEnemy_Black OtherActor)
    (Variables|Default|SetIsBlackPushed? true)
    (Physics|SetSimulatePhysics OtherComp true)
    (Physics|AddForce OtherComp (* (* (Transformation|GetActorForwardVector) (Variables|Default|GetPushForce)) 1e+06) "None" false)
    (else
      (Physics|SetSimulatePhysics OtherComp false))))

(event OnComponentBeginOverlap(RedPushCol)
  (params (OverlappedComponent :type Primitive%20Component%20Object%20Reference) (OtherActor :type Actor%20Object%20Reference) (OtherComp :type Primitive%20Component%20Object%20Reference) (OtherBodyIndex :type Integer) (bFromSweep :type Boolean) (SweepResult :type Hit%20Result%20Structure%20%28by%20ref%29))
  ;[0.15 0.15 0.15 0.5] PUSH RED
  (if (Actor|ActorHasTag OtherActor (Variables|Default|GetTagRed))
    (Variables|Default|SetEnemy_Red OtherActor)
    (Variables|Default|SetIsRedPushed? true)
    (Physics|SetSimulatePhysics OtherComp true)
    (Physics|AddForce OtherComp (* (* (Transformation|GetActorForwardVector) (Variables|Default|GetPushForce)) 1e+06) "None" false)
    (else
      (Physics|SetSimulatePhysics OtherComp false))))

(event Custom|TurnVertically
  ;[0.15 0.15 0.15 0.5] Vertical Turn
  (if (Variables|Default|GetIsUp?)
    (CallFunction|FlipFlopTurn)
    (Variables|Default|SetIsUp? false)
    (Variables|Default|SetCanHorizontalTurn true)
    (Variables|Default|SetCanCollect? true)
    (else
      (CallFunction|FlipFlopTurn)
      (Variables|Default|SetIsUp? true)
      (Variables|Default|SetCanHorizontalTurn false)
      (Variables|Default|SetCanCollect? false))))

(event Custom|FlipFlopTurn
  ;[0.15 0.15 0.15 0.5] Vertical Turn
  (Utilities|FlowControl|FlipFlop
    (:A
      (bind _verticalrotate (Timeline|VerticalRotate Play)
        (:Update
          (Transformation|SetRelativeRotation (Variables|Default|GetCube) (Math|Rotator|MakeRotator 0.0 _verticalrotate 0.0) false false))))
    (:B
      (Timeline|VerticalRotate Reverse))))

(event Custom|ReleaseRedTin
  (if (Variables|Default|GetisRedCollected?)
    (Variables|Default|SetisRedCollected? false)
    (Variables|Default|SetIsRedFull? false)
    (Variables|Default|SetCanVertTurn? true)
    (bind _asbp_mag_red (Utilities|Casting|CastToBP_Mag_Red (Variables|Default|GetCollectedRedTin)))
    (Utilities|IsValid _asbp_mag_red
      (:Is%20Valid
        (Default|Release _asbp_mag_red)))))

(event Custom|ReleaseBlackTin)

(event Input|EnhancedActionEvents|EnhancedInputActionIA_MagnetMove
  (params (ActionValue :type Vector%202D%20Structure) (ElapsedSeconds :type Float%20%28double-precision%29) (TriggeredSeconds :type Float%20%28double-precision%29) (InputAction :type Input%20Action%20Object%20Reference :default "/Game/_Game/Input/IA_MagnetMove.IA_MagnetMove"))
  (bind _returnvalue (Pawn|GetControlRotation :!class /Script/Engine.Pawn))
  ;[0.15 0.15 0.15 0.5] Movement
  (if (Variables|Default|GetCanMove?)
    (Pawn|Input|AddMovementInput (Math|Vector|GetRightVector (Math|Rotator|MakeRotator (.roll _returnvalue) 0.0 (.yaw _returnvalue))) (.x ActionValue) false)
    (Pawn|Input|AddMovementInput (Math|Vector|GetForwardVector (Math|Rotator|MakeRotator 0.0 0.0 (.yaw _returnvalue))) (.y ActionValue) false)))

(event Input|EnhancedActionEvents|EnhancedInputActionIA_MagnetLook
  (params (ActionValue :type Vector%202D%20Structure) (ElapsedSeconds :type Float%20%28double-precision%29) (TriggeredSeconds :type Float%20%28double-precision%29) (InputAction :type Input%20Action%20Object%20Reference :default "/Game/_Game/Input/IA_MagnetLook.IA_MagnetLook"))
  ;[0.15 0.15 0.15 0.5] Look
  (Pawn|Input|AddControllerYawInput (Math|Float|Clamp(Float) (.x ActionValue) -0.5 0.5)))

(event Input|EnhancedActionEvents|EnhancedInputActionIA_MagnetTurn
  (params (ActionValue :type Boolean) (ElapsedSeconds :type Float%20%28double-precision%29) (TriggeredSeconds :type Float%20%28double-precision%29) (InputAction :type Input%20Action%20Object%20Reference :default "/Game/_Game/Input/IA_MagnetTurn.IA_MagnetTurn"))
  ;[0.15 0.15 0.15 0.5] Horizontal Turn
  (if (Variables|Default|GetCanHorizontalTurn)
    (Utilities|FlowControl|FlipFlop
      (:A
        (bind _rotateintime (Timeline|TRotator Play)
          (:Update
            (Transformation|SetRelativeRotation (Variables|Default|GetCube) (Math|Rotator|MakeRotator 0.0 0.0 _rotateintime) false false))))
      (:B
        (Timeline|TRotator Reverse)))))

(event Input|EnhancedActionEvents|EnhancedInputActionIA_MagnetTurnVertical
  (params (ActionValue :type Boolean) (ElapsedSeconds :type Float%20%28double-precision%29) (TriggeredSeconds :type Float%20%28double-precision%29) (InputAction :type Input%20Action%20Object%20Reference :default "/Game/_Game/Input/IA_MagnetTurnVertical.IA_MagnetTurnVertical"))
  ;[0.15 0.15 0.15 0.5] Vertical Turn
  (if (Variables|Default|GetCanVertTurn?)
    (CallFunction|TurnVertically)))

(event EventBeginPlay
  ;[0.15 0.15 0.15 0.5] Initiate
  (bind _asplayer_controller (Utilities|Casting|CastToPlayerController (Pawn|GetController)))
  (Utilities|IsValid (PlayerController|LocalPlayerSubsystems|GetEnhancedInputLocalPlayerSubsystem _asplayer_controller)
    (:Is%20Valid
      (Input|AddMappingContext (PlayerController|LocalPlayerSubsystems|GetEnhancedInputLocalPlayerSubsystem _asplayer_controller) "/Game/_Game/Input/IMC_Magnet.IMC_Magnet" 0 "(bIgnoreAllPressedKeysUntilRelease=True,bForceImmediately=False,bNotifyUserSettings=False)")
      (Components|Activation|SetActive (Variables|Default|GetBPC_Magnet) true false))))

(fn ConstructionScript)