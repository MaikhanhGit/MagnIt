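; BPC_Magnet is an actor component that makes its owner act as a magnet on nearby actors.
; A looping timer started at BeginPlay runs a single-hit sphere trace at the owner's location, sized by MagneticRadius and debug-drawn for one frame.
; If the hit actor implements BPI_MagneticField, it is stored as TargetActor and sent AttrackMessage; otherwise the target is cleared.
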(event Custom|UpdateMagneticField
  (CallFunction|GetMagneticField))

(event EventBeginPlay
  (Utilities|Time|SetTimerbyEvent (delegate Custom|UpdateMagneticField) 0.2 true))

(fn GetMagneticField
  (bind _returnvalue (Components|GetOwner))
  (bind _returnvalue_2 (Transformation|GetActorLocation _returnvalue))
  (bind (_outhit _returnvalue_3) (Collision|SphereTraceByChannel _returnvalue_2 _returnvalue_2 (Variables|Default|GetMagneticRadius) "TraceTypeQuery3" false 0 "ForOneFrame"))
  (if _returnvalue_3
    (if (Utilities|DoesObjectImplementInterface (.HitActor (Collision|BreakHitResult _outhit)) "/Game/_Game/MagnetGame/Magnet/BPI_MagneticField.BPI_MagneticField_C")
      (bind _output_get (Variables|Default|SetTargetActor (.HitActor (Collision|BreakHitResult _outhit))))
      (Class|BPIMagneticField|Attrack(Message) _output_get)
      (else
        (Variables|Default|SetTargetActor 0)))
    (else
      (Variables|Default|SetTargetActor 0))))