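; BPC_RedMagnet is an actor component that gives its owner a red magnetic field for the magnet game.
; A looping timer started on BeginPlay periodically runs a zero-length sphere trace at the owner's location, with debug drawing on.
; If the single hit actor implements BPI_RedMagneticField, it is stored as TargetActor and sent RedAttrackMessage; otherwise TargetActor is cleared.
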(event Custom|UpdateRedMagneticField
  (CallFunction|GetRedMagneticField))

(event EventBeginPlay
  (Utilities|Time|SetTimerbyEvent (delegate Custom|UpdateRedMagneticField) 0.2 true))

(fn GetRedMagneticField
  (bind _returnvalue (Components|GetOwner))
  (bind _returnvalue_2 (Transformation|GetActorLocation _returnvalue))
  (bind (_outhit _returnvalue_3) (Collision|SphereTraceByChannel _returnvalue_2 _returnvalue_2 (Variables|Default|GetRedMagneticRadius) "TraceTypeQuery4" false 0 "ForOneFrame"))
  (if _returnvalue_3
    (if (Utilities|DoesObjectImplementInterface (.HitActor (Collision|BreakHitResult _outhit)) "/Game/_Game/MagnetGame/Magnet/BPI_RedMagneticField.BPI_RedMagneticField_C")
      (bind _output_get (Variables|Default|SetTargetActor (.HitActor (Collision|BreakHitResult _outhit))))
      (Class|BPIRedMagneticField|RedAttrack(Message) _output_get)
      (else
        (Variables|Default|SetTargetActor 0)))
    (else
      (Variables|Default|SetTargetActor 0))))