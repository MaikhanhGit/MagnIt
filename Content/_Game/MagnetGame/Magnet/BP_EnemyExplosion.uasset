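; BP_EnemyExplosion is an actor in the magnet game that can be pulled into the player; despite its name, its graph holds no explosion logic.
; Its Attrack event checks that the player character is a BP_Magnet with an active BPC_Magnet component.
; It then disables mesh collision, eases the root toward the player's location sampled by MoveComponentTo, and destroys itself when the short move completes.
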(event EventBeginPlay)

(event Collision|EventActorBeginOverlap
  (params (OtherActor :type Actor%20Object%20Reference)))

(event EventTick
  (params (DeltaSeconds :type Float%20%28single-precision%29)))

(event EventAttrack
  (bind _asbp_magnet (Utilities|Casting|CastToBP_Magnet (Game|GetPlayerCharacter 0)))
  (Utilities|IsValid (Actor|GetComponentbyClass _asbp_magnet "/Game/_Game/MagnetGame/Magnet/BPC_Magnet.BPC_Magnet_C")
    (:Is%20Valid
      (if (Components|Activation|IsActive (Actor|GetComponentbyClass _asbp_magnet "/Game/_Game/MagnetGame/Magnet/BPC_Magnet.BPC_Magnet_C"))
        (Collision|SetCollisionEnabled (Variables|Default|GetStaticMesh) "NoCollision")
        (Components|MoveComponentTo (Variables|Default|GetDefaultSceneRoot) (Transformation|GetActorLocation _asbp_magnet) "0, 0, 0" false true 0.4 false)
        (Actor|DestroyActor)))))

(fn ConstructionScript)