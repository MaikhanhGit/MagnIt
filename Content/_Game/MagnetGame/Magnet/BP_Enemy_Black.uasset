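; BP_Enemy_Black is an enemy in the magnet game that the player's black magnet pulls in.
; Its BlackAttrack event checks that the player's BP_Magnet has an active BPC_BlackMagnet component and a valid BlackDestCol.
; It then disables the cube's collision and moves its root to that destination's transform over a short interval.
; BeginPlay is empty and a looping timer node is left unwired.
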(event EventBlackAttrack
  (bind _asbp_magnet (Utilities|Casting|CastToBP_Magnet (Game|GetPlayerCharacter 0)))
  (Utilities|IsValid (Actor|GetComponentbyClass _asbp_magnet "/Game/_Game/MagnetGame/Magnet/BPC_BlackMagnet.BPC_BlackMagnet_C")
    (:Is%20Valid
      (if (Components|Activation|IsActive (Actor|GetComponentbyClass _asbp_magnet "/Game/_Game/MagnetGame/Magnet/BPC_BlackMagnet.BPC_BlackMagnet_C"))
        (Utilities|IsValid (Variables|/Game/_Game/MagnetGame/BP_Magnet.BP_Magnet_C|GetBlackDestCol _asbp_magnet)
          (:Is%20Valid
            (Collision|SetCollisionEnabled (Variables|Default|GetCube) "NoCollision")
            (Components|MoveComponentTo (Variables|Default|GetDefaultSceneRoot) (Transformation|GetWorldLocation (Variables|/Game/_Game/MagnetGame/BP_Magnet.BP_Magnet_C|GetBlackDestCol _asbp_magnet)) (Transformation|GetWorldRotation (Variables|/Game/_Game/MagnetGame/BP_Magnet.BP_Magnet_C|GetBlackDestCol _asbp_magnet)) false false 0.3 false)))))))

(event EventBeginPlay)

(fn ConstructionScript)