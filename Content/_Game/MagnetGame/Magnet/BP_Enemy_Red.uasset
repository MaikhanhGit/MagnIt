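; BP_Enemy_Red is a red enemy in the magnet game that is pulled toward the player magnet's Black object.
; The RedAttrack event activates it when the player's BP_Magnet has an active BPC_RedMagnet.
; While active, Tick swaps the cube to a deactivated material if red is pushed.
; Otherwise it enables collision and runs nested timelines that lerp location and rotation toward Black through MoveComponentTo.
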(event EventBeginPlay)

(event EventRedAttrack
  (if (not (Variables|Default|GetIsActivated?))
    (bind _asbp_magnet (Utilities|Casting|CastToBP_Magnet (Game|GetPlayerCharacter 0)))
    (Utilities|IsValid (Actor|GetComponentbyClass _asbp_magnet "/Game/_Game/MagnetGame/Magnet/BPC_RedMagnet.BPC_RedMagnet_C")
      (:Is%20Valid
        (bind _output_get (Variables|Default|SetTargetObj _asbp_magnet))
        (if (Components|Activation|IsActive (Actor|GetComponentbyClass _asbp_magnet "/Game/_Game/MagnetGame/Magnet/BPC_RedMagnet.BPC_RedMagnet_C"))
          (Utilities|IsValid _output_get
            (:Is%20Valid
              (Variables|Default|SetIsActivated? true))))))))

(event EventTick
  (params (DeltaSeconds :type Float%20%28single-precision%29))
  (bind _targetobj (Variables|Default|GetTargetObj))
  (bind _defaultsceneroot (Variables|Default|GetDefaultSceneRoot))
  (bind _black (Variables|/Game/_Game/MagnetGame/BP_Magnet.BP_Magnet_C|GetBlack _targetobj))
  (if (Variables|Default|GetIsActivated?)
    (if (Variables|/Game/_Game/MagnetGame/BP_Magnet.BP_Magnet_C|GetIsRedPushed? (Variables|Default|GetTargetObj))
      (Rendering|Material|SetMaterial (Variables|Default|GetCube) 0 "/Game/_Game/Materials/M_DeactivatedRed.M_DeactivatedRed")
      (else
        (Collision|SetCollisionEnabled (Variables|Default|GetCube) "QueryAndPhysics")
        (Utilities|IsValid _black
          (:Is%20Valid
            (bind _enemymove (Timeline|EnemyMove Play)
              (:Update
                (bind _turnlerp (Timeline|TurnLerp Play)
                  (:Update
                    (Components|MoveComponentTo _defaultsceneroot (Math|Vector|Lerp(Vector) (Transformation|GetWorldLocation (Variables|Default|GetDefaultSceneRoot)) (Transformation|GetWorldLocation _black) _enemymove) (Math|Rotator|Lerp(Rotator) (Transformation|GetWorldRotation _defaultsceneroot) (Transformation|GetWorldRotation _black) _turnlerp) false false 0.3 false)))))))))))

(fn ConstructionScript)