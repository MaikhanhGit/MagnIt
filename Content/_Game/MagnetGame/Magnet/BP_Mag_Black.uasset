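; BP_Mag_Black is the black magnet object in the magnet game, which gets pulled onto the player's BP_Magnet.
; RedAttack requires an active BPC_BlackMagnet and nothing black collected, then moves the object to BlackDestCol and flags it collected.
; A looping timer at AttrackFrequency keeps re-moving it to that target with collision off.
; Release zeroes velocity and enables physics, but does not clear the timer or flag.
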(event Custom|MagIsActivated
  (bind _target (Variables|Default|GetTarget))
  (Collision|SetCollisionEnabled (Variables|Default|GetCube) "NoCollision")
  (Components|MoveComponentTo (Variables|Default|GetDefaultSceneRoot) (Transformation|GetWorldLocation _target) (Transformation|GetWorldRotation _target) false false 0.5 false))

(event Custom|Release
  (Physics|SetPhysicsLinearVelocity (Variables|Default|GetCube) "0, 0, 0" false "None")
  (Physics|SetSimulatePhysics (Variables|Default|GetCube) true)
  (Development|PrintString "Black Released"))

(event EventBeginPlay)

(event EventRedAttrack
  (bind _asbp_magnet (Utilities|Casting|CastToBP_Magnet (Game|GetPlayerCharacter 0)))
  (Utilities|IsValid (Actor|GetComponentbyClass _asbp_magnet "/Game/_Game/MagnetGame/Magnet/BPC_BlackMagnet.BPC_BlackMagnet_C")
    (:Is%20Valid
      (if (Components|Activation|IsActive (Actor|GetComponentbyClass _asbp_magnet "/Game/_Game/MagnetGame/Magnet/BPC_BlackMagnet.BPC_BlackMagnet_C"))
        (bind _output_get (Variables|Default|SetPlayerBP _asbp_magnet))
        (if (not (Variables|/Game/_Game/MagnetGame/BP_Magnet.BP_Magnet_C|GetisBlackCollected? _output_get))
          (Utilities|IsValid (Variables|/Game/_Game/MagnetGame/BP_Magnet.BP_Magnet_C|GetBlackDestCol _output_get)
            (:Is%20Valid
              (Variables|Default|SetTarget (Variables|/Game/_Game/MagnetGame/BP_Magnet.BP_Magnet_C|GetBlackDestCol _output_get))
              (Collision|SetCollisionEnabled (Variables|Default|GetCube) "QueryOnly")
              (Components|MoveComponentTo (Variables|Default|GetDefaultSceneRoot) (Transformation|GetWorldLocation (Variables|Default|GetTarget)) (Transformation|GetWorldRotation (Variables|Default|GetTarget)) false false 0.5 false)
              (Variables|/Game/_Game/MagnetGame/BP_Magnet.BP_Magnet_C|SetisBlackCollected? (Variables|Default|GetPlayerBP) true)
              (Utilities|Time|SetTimerbyEvent (delegate Custom|MagIsActivated) (Variables|Default|GetAttrackFrequency) true))))))))

(fn ConstructionScript)