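; BP_BoxSpawner is a magnet-mechanics actor that spawns a BP_BlackBox at its own location and rotation on BeginPlay.
; SpawnBox adjusts for collisions but always spawns, stores the box as SpawnItem and hands it a reference back to the spawner.
; Tick is empty, and a disconnected respawn check on destruction never runs, so this Blueprint itself only triggers the initial spawn.
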(event Custom|SpawnBox
  (bind _returnvalue (Transformation|GetActorTransform))
  (bind _returnvalue_2 (Game|SpawnActorfromClass "/Game/_Game/MagnetMechanics/Magnets/BP_BlackBox.BP_BlackBox_C" (Math|Transform|MakeTransform (.location _returnvalue) (.rotation _returnvalue) "1.000000,1.000000,1.000000") "AdjustIfPossibleButAlwaysSpawn" "MultiplyWithRoot" 0 0))
  (bind _output_get (Variables|Default|SetSpawnItem _returnvalue_2))
  (Variables|/Game/_Game/MagnetMechanics/Magnets/BP_BlackBox.BP_BlackBox_C|SetBoxSpawner _output_get self))

(event EventBeginPlay
  (CallFunction|SpawnBox))

(event EventTick
  (params (DeltaSeconds :type Float%20%28single-precision%29)))

(fn ConstructionScript)