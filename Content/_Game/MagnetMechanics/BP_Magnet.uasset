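; BP_Magnet is the player character, a two-pole red/black magnet that moves, sprints and flips to change its forward pole.
; Timelines rotate the body horizontally or vertically (upright locks movement), while Tick activates the magnet component for the forward color.
; Colored overlap volumes push same-color enemies and boxes with physics forces and track tins for release.
; Contact with explosive enemies breaks the magnet apart, calls Lose and reloads SandBox.
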(event OnComponentBeginOverlap(RdPushCol)
  (params (OverlappedComponent :type Primitive%20Component%20Object%20Reference) (OtherActor :type Actor%20Object%20Reference) (OtherComp :type Primitive%20Component%20Object%20Reference) (OtherBodyIndex :type Integer) (bFromSweep :type Boolean) (SweepResult :type Hit%20Result%20Structure%20%28by%20ref%29))
  ;[0.15 0.15 0.15 0.5] Push Red Enemy
  (if (Actor|ActorHasTag OtherActor (Variables|Default|GetTagRed))
    (bind _output_get (Variables|Default|SetEnemy_Red OtherActor))
    (bind _asbp_enemy_red (Utilities|Casting|CastToBP_Enemy_Red _output_get))
    (Variables|/Game/_Game/MagnetMechanics/Magnets/BP_Enemy_Red.BP_Enemy_Red_C|SetisPushed? _asbp_enemy_red true)
    (Physics|SetSimulatePhysics OtherComp true)
    (Physics|AddForce OtherComp (* (* (Transformation|GetActorForwardVector) (Variables|Default|GetPushForce)) 1e+06) "None" false)
    (else
      ;[0.15 0.15 0.15 0.5] Push Red Box
      (if (Actor|ActorHasTag OtherActor "RedMag")
        (bind _asbp_magnet_red (Utilities|Casting|CastToBP_Magnet_Red OtherActor))
        (Variables|/Game/_Game/MagnetMechanics/Magnets/BP_Magnet_Red.BP_Magnet_Red_C|SetisPushed? _asbp_magnet_red true)
        (Collision|SetCollisionEnabled OtherComp "QueryAndPhysics")
        (Physics|SetSimulatePhysics OtherComp true)
        (Physics|AddForce OtherComp (* (* (Transformation|GetActorForwardVector) (Variables|Default|GetPushForce)) 1e+06) "None" false)))))

(event OnComponentBeginOverlap(BlackDestCol)
  (params (OverlappedComponent :type Primitive%20Component%20Object%20Reference) (OtherActor :type Actor%20Object%20Reference) (OtherComp :type Primitive%20Component%20Object%20Reference) (OtherBodyIndex :type Integer) (bFromSweep :type Boolean) (SweepResult :type Hit%20Result%20Structure%20%28by%20ref%29))
  ;[0.15 0.15 0.15 0.5] Check If Holding Anything
  (if (Actor|ActorHasTag OtherActor "TinBlack")
    (Variables|Default|SetCollectedBlackTin OtherActor)))

(event OnComponentBeginOverlap(RedDestCol)
  (params (OverlappedComponent :type Primitive%20Component%20Object%20Reference) (OtherActor :type Actor%20Object%20Reference) (OtherComp :type Primitive%20Component%20Object%20Reference) (OtherBodyIndex :type Integer) (bFromSweep :type Boolean) (SweepResult :type Hit%20Result%20Structure%20%28by%20ref%29))
  ;[0.15 0.15 0.15 0.5] Check If Holding Anything
  (if (Actor|ActorHasTag OtherActor "TinRed")
    (Variables|Default|SetCollectedRedTin OtherActor)))

(event OnComponentBeginOverlap(PlayerKillCollision)
  (params (OverlappedComponent :type Primitive%20Component%20Object%20Reference) (OtherActor :type Actor%20Object%20Reference) (OtherComp :type Primitive%20Component%20Object%20Reference) (OtherBodyIndex :type Integer) (bFromSweep :type Boolean) (SweepResult :type Hit%20Result%20Structure%20%28by%20ref%29))
  ;[0.15 0.15 0.15 0.5] Enemies Enter - Player's Killed
  (if (Actor|ActorHasTag OtherActor "ExplosionRed")
    (bind _asbp_enemy_red (Utilities|Casting|CastToBP_Enemy_Red OtherActor))
    (Physics|SetSimulatePhysics (Variables|/Game/_Game/MagnetMechanics/Magnets/BP_Enemy_Red.BP_Enemy_Red_C|GetCube _asbp_enemy_red) true)
    (Class|PrimitiveComponent|AddForceatLocation (Variables|/Game/_Game/MagnetMechanics/Magnets/BP_Enemy_Red.BP_Enemy_Red_C|GetCube _asbp_enemy_red) (* (* (Transformation|GetActorUpVector) (Variables|Default|GetLosePushForce)) 1e+06) (Transformation|GetWorldLocation (Variables|Collision|GetCapsuleComponent)) "None")
    (Default|StartEarlyExplosion _asbp_enemy_red)
    (CallFunction|StartLoseState)
    (elif (Actor|ActorHasTag OtherActor "ExplosionBlack")
      (bind _asbp_enemy_black (Utilities|Casting|CastToBP_Enemy_Black OtherActor))
      (Physics|SetSimulatePhysics (Variables|/Game/_Game/MagnetMechanics/Magnets/BP_Enemy_Black.BP_Enemy_Black_C|GetCube _asbp_enemy_black) true)
      (Class|PrimitiveComponent|AddForceatLocation (Variables|/Game/_Game/MagnetMechanics/Magnets/BP_Enemy_Black.BP_Enemy_Black_C|GetCube _asbp_enemy_black) (* (* (Transformation|GetActorUpVector) (Variables|Default|GetLosePushForce)) 1e+06) (Transformation|GetWorldLocation (Variables|Collision|GetCapsuleComponent)) "None")
      (Default|StartExplosion _asbp_enemy_black)
      (CallFunction|StartLoseState)
      (elif (Actor|ActorHasTag OtherActor "Grinder")
        _))))

(event OnComponentBeginOverlap(BlkPushCol)
  (params (OverlappedComponent :type Primitive%20Component%20Object%20Reference) (OtherActor :type Actor%20Object%20Reference) (OtherComp :type Primitive%20Component%20Object%20Reference) (OtherBodyIndex :type Integer) (bFromSweep :type Boolean) (SweepResult :type Hit%20Result%20Structure%20%28by%20ref%29))
  ;[0.15 0.15 0.15 0.5] Push Black Enemy
  (if (Actor|ActorHasTag OtherActor (Variables|Default|GetTagBlack))
    (bind _output_get (Variables|Default|SetEnemy_Black OtherActor))
    (bind _asbp_enemy_black (Utilities|Casting|CastToBP_Enemy_Black _output_get))
    (Variables|/Game/_Game/MagnetMechanics/Magnets/BP_Enemy_Black.BP_Enemy_Black_C|SetisPushed? _asbp_enemy_black true)
    (Physics|SetSimulatePhysics OtherComp true)
    (Physics|AddForce OtherComp (* (* (Transformation|GetActorForwardVector) (Variables|Default|GetPushForce)) 1e+06) "None" false)
    (else
      ;[0.15 0.15 0.15 0.5] Push Black Box
      (if (Actor|ActorHasTag OtherActor "BlackMag")
        (bind _asbp_magnet_black (Utilities|Casting|CastToBP_Magnet_Black OtherActor))
        (Variables|/Game/_Game/MagnetMechanics/Magnets/BP_Magnet_Black.BP_Magnet_Black_C|SetisPushed? _asbp_magnet_black true)
        (Collision|SetCollisionEnabled OtherComp "QueryAndPhysics")
        (Physics|SetSimulatePhysics OtherComp true)
        (Physics|AddForce OtherComp (* (* (Transformation|GetActorForwardVector) (Variables|Default|GetPushForce)) 1e+06) "None" false)))))

(event Custom|TurnVertically
  ;[0.15 0.15 0.15 0.5] Vertical Turn
  (if (Variables|Default|GetIsUp?)
    (CallFunction|FlipFlopTurn)
    (Variables|Default|SetIsUp? false)
    (Variables|Default|SetCanHorizontalTurn true)
    (Variables|Default|SetCanMove? true)
    (else
      (CallFunction|FlipFlopTurn)
      (Variables|Default|SetIsUp? true)
      (Variables|Default|SetCanHorizontalTurn false)
      (Variables|Default|SetCanMove? false))))

(event Custom|FlipFlopTurn
  ;[0.15 0.15 0.15 0.5] Vertical Turn
  (Utilities|FlowControl|FlipFlop
    (:A
      (bind _verticalrotate (Timeline|VerticalRotate Play)
        (:Update
          (if (Variables|Default|GetisRedForward?)
            (Transformation|SetRelativeRotation (Variables|Default|GetCube) (Math|Rotator|MakeRotator 0.0 (* _verticalrotate -9e+01) 0.0) false false)
            (else
              (Transformation|SetRelativeRotation (Variables|Default|GetCube) (Math|Rotator|MakeRotator 0.0 (* _verticalrotate -9e+01) -1.8e+02) false false))))))
    (:B
      (Timeline|VerticalRotate Reverse))))

(event Custom|ReleaseRedTin
  ;[0.15 0.15 0.15 0.5] Release
  (bind _asbp_tin_red (Utilities|Casting|CastToBP_Tin_Red (Variables|Default|GetCollectedRedTin)))
  (Utilities|IsValid _asbp_tin_red
    (:Is%20Valid
      (Default|Release _asbp_tin_red)
      (Variables|Default|SetisRedCollected? false))))

(event Custom|ReleaseBlackTin
  ;[0.15 0.15 0.15 0.5] Release
  (bind _asbp_tin_black (Utilities|Casting|CastToBP_Tin_Black (Variables|Default|GetCollectedBlackTin)))
  (Utilities|IsValid _asbp_tin_black
    (:Is%20Valid
      (Default|Release _asbp_tin_black)
      (Variables|Default|SetisBlackCollected? false))))

(event Custom|StartLoseState
  (bind _red (Variables|Default|GetRed))
  (bind _black (Variables|Default|GetBlack))
  ;[0.15 0.15 0.15 0.5] Start LOSE
  (Components|Activation|SetActive (Variables|Default|GetExplosionNia) true false)
  (Physics|SetSimulatePhysics _red true)
  (Physics|AddForce _red (* (Transformation|GetActorForwardVector) (Variables|Default|GetBreakingForce)) "None" false)
  (Physics|SetSimulatePhysics _black true)
  (Physics|AddForce _black (* (Transformation|GetActorForwardVector) (Variables|Default|GetBreakingForceNegative)) "None" false)
  (Utilities|FlowControl|Delay (Variables|Default|GetLoseDelay))
  (bind _asmagnet_player_controller (Utilities|Casting|CastToMagnetPlayerController (Game|GetPlayerController 0)))
  (Default|Lose _asmagnet_player_controller)
  (Utilities|FlowControl|Delay 1.0)
  (Game|OpenLevel(byName) "SandBox"))

(event Custom|RotateArt
  (Transformation|AddRelativeRotation (Variables|Default|GetBottomArt) "0.000000,5.000000,0.000000" false false))

(event Input|EnhancedActionEvents|EnhancedInputActionIA_MagnetMove
  (params (ActionValue :type Vector%202D%20Structure) (ElapsedSeconds :type Float%20%28double-precision%29) (TriggeredSeconds :type Float%20%28double-precision%29) (InputAction :type Input%20Action%20Object%20Reference :default "/Game/_Game/Input/IA_MagnetMove.IA_MagnetMove"))
  (bind _returnvalue (Pawn|GetControlRotation :!class /Script/Engine.Pawn))
  ;[0.15 0.15 0.15 0.5] Movement
  (if (Variables|Default|GetCanMove?)
    (Pawn|Input|AddMovementInput (Math|Vector|GetRightVector (Math|Rotator|MakeRotator (.roll _returnvalue) 0.0 (.yaw _returnvalue))) (* (.x ActionValue) (Variables|Default|GetSprintMultiply)) false)
    (Pawn|Input|AddMovementInput (Math|Vector|GetForwardVector (Math|Rotator|MakeRotator 0.0 0.0 (.yaw _returnvalue))) (* (.y ActionValue) (Variables|Default|GetSprintMultiply)) false)))

(event Input|EnhancedActionEvents|EnhancedInputActionIA_MagnetLook
  (params (ActionValue :type Vector%202D%20Structure) (ElapsedSeconds :type Float%20%28double-precision%29) (TriggeredSeconds :type Float%20%28double-precision%29) (InputAction :type Input%20Action%20Object%20Reference :default "/Game/_Game/Input/IA_MagnetLook.IA_MagnetLook"))
  ;[0.15 0.15 0.15 0.5] Look
)

(event Input|EnhancedActionEvents|EnhancedInputActionIA_MagnetSprint
  (params (ActionValue :type Boolean) (ElapsedSeconds :type Float%20%28double-precision%29) (TriggeredSeconds :type Float%20%28double-precision%29) (InputAction :type Input%20Action%20Object%20Reference :default "/Game/_Game/Input/IA_MagnetSprint.IA_MagnetSprint"))
  (:Triggered
    (if (Variables|Default|GetCanMove?)
      (CallFunction|Sprint)))
  (:Completed
    (CallFunction|StopSprint)))

(event Input|EnhancedActionEvents|EnhancedInputActionIA_MagnetTurnVertical
  (params (ActionValue :type Boolean) (ElapsedSeconds :type Float%20%28double-precision%29) (TriggeredSeconds :type Float%20%28double-precision%29) (InputAction :type Input%20Action%20Object%20Reference :default "/Game/_Game/Input/IA_MagnetTurnVertical.IA_MagnetTurnVertical"))
  ;[0.15 0.15 0.15 0.5] Vertical Turn
  (if (Variables|Default|GetCanVertTurn?)
    (CallFunction|TurnVertically)))

(event Input|EnhancedActionEvents|EnhancedInputActionIA_MagnetTurn
  (params (ActionValue :type Boolean) (ElapsedSeconds :type Float%20%28double-precision%29) (TriggeredSeconds :type Float%20%28double-precision%29) (InputAction :type Input%20Action%20Object%20Reference :default "/Game/_Game/Input/IA_MagnetTurn.IA_MagnetTurn"))
  ;[0.15 0.15 0.15 0.5] Horizontal Turn Original
  (if (Variables|Default|GetCanHorizontalTurn)
    (Utilities|FlowControl|FlipFlop
      (:A
        (Variables|Default|SetisRedForward? false)
        (bind _rotateintime (Timeline|TRotator Play)
          (:Update
            (Transformation|SetRelativeRotation (Variables|Default|GetCube) (Math|Rotator|MakeRotator 0.0 0.0 (* _rotateintime -1.8e+02)) false false))))
      (:B
        (Variables|Default|SetisRedForward? true)
        (Timeline|TRotator Reverse)))))

(event EventBeginPlay
  ;[0.15 0.15 0.15 0.5] Initiate
  (bind _asplayer_controller (Utilities|Casting|CastToPlayerController (Pawn|GetController)))
  (Utilities|IsValid (PlayerController|LocalPlayerSubsystems|GetEnhancedInputLocalPlayerSubsystem _asplayer_controller)
    (:Is%20Valid
      (Input|AddMappingContext (PlayerController|LocalPlayerSubsystems|GetEnhancedInputLocalPlayerSubsystem _asplayer_controller) "/Game/_Game/Input/IMC_Magnet.IMC_Magnet" 0 "(bIgnoreAllPressedKeysUntilRelease=True,bForceImmediately=False,bNotifyUserSettings=False)")
      (Components|Activation|SetActive (Variables|Default|GetBPC_Magnet) false false)
      (Components|Activation|SetActive (Variables|Default|GetBPC_RedMagnet) true false)
      (Components|Activation|SetActive (Variables|Default|GetBPC_BlackMagnet) true false)
      (Components|Activation|SetActive (Variables|Default|GetExplosionNia) false false)
      (Components|Activation|SetActive (Variables|Default|GetBPC_MagTin_Black) true false)
      (Components|Activation|SetActive (Variables|Default|GetBPC_MagTin_Red) true false)
      (Variables|Default|SetDefaultMaxWalkSpeed (Variables|/Script/Engine.CharacterMovementComponent|GetMaxWalkSpeed (Variables|Character|GetCharacterMovement))))))

(event EventTick
  (params (DeltaSeconds :type Float%20%28single-precision%29))
  (if (Variables|Default|GetisRedForward?)
    (Components|Activation|SetActive (Variables|Default|GetBPC_RedMagnet) true false)
    (Components|Activation|SetActive (Variables|Default|GetBPC_BlackMagnet) false false)
    (else
      (Components|Activation|SetActive (Variables|Default|GetBPC_RedMagnet) false false)
      (Components|Activation|SetActive (Variables|Default|GetBPC_BlackMagnet) true false))))

(fn ConstructionScript)

(fn Sprint
  (Variables|Default|SetSprintMultiply 1e+06))

(fn StopSprint
  (Variables|Default|SetSprintMultiply 1e+01))