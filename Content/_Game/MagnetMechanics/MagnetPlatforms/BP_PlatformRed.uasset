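; Red magnet platform that shuttles between its start and EndPoint and catches a BP_Magnet player whose black side is up.
; A FlipFlop-driven timeline moves the mesh back and forth with a pause between trips.
; On a Black-tagged overlap, a PhysicsHandle grabs the player's cube, then Tick snaps the player to the trigger box, locking movement and disabling magnet collision.
; When black is no longer up, it releases, unlocks and turns the player.
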(event OnComponentBeginOverlap(BoxCollision)
  (params (OverlappedComponent :type Primitive%20Component%20Object%20Reference) (OtherActor :type Actor%20Object%20Reference) (OtherComp :type Primitive%20Component%20Object%20Reference) (OtherBodyIndex :type Integer) (bFromSweep :type Boolean) (SweepResult :type Hit%20Result%20Structure%20%28by%20ref%29))
  (if (Components|ComponentHasTag OtherComp "Black")
    (bind _asbp_magnet (Utilities|Casting|CastToBP_Magnet OtherActor))
    (bind _output_get (Variables|Default|SetPlayer _asbp_magnet))
    (if (Variables|/Game/_Game/MagnetMechanics/BP_Magnet.BP_Magnet_C|GetIsBlackUp? _output_get)
      (Class|PhysicsHandleComponent|GrabComponentatLocation (Variables|Default|GetPhysicsHandle) (Variables|/Game/_Game/MagnetMechanics/BP_Magnet.BP_Magnet_C|GetCube (Variables|Default|GetPlayer)) "None" (Transformation|GetWorldLocation (Variables|/Game/_Game/MagnetMechanics/BP_Magnet.BP_Magnet_C|GetCube (Variables|Default|GetPlayer))))
      (Variables|Default|SetIsHolding? true))))

(event Custom|AddForceToObj)

(event Custom|TurnOffCollisions
  (bind _player (Variables|Default|GetPlayer))
  (Collision|SetCollisionEnabled (Variables|/Game/_Game/MagnetMechanics/BP_Magnet.BP_Magnet_C|GetBlack _player) "NoCollision")
  (Collision|SetCollisionEnabled (Variables|/Game/_Game/MagnetMechanics/BP_Magnet.BP_Magnet_C|GetRed _player) "NoCollision"))

(event Custom|TurnOnCollision
  (Default|RedForwardTurnVertically (Variables|Default|GetPlayer)))

(event EventBeginPlay
  (Components|Timeline|SetPlayRate (Variables|Default|GetMovement) (Variables|Default|GetPlayRate))
  (Utilities|FlowControl|FlipFlop :!label _label
    (:A
      (bind _movement (Timeline|Movement Play)
        (:Update
          (Transformation|SetRelativeLocation (Variables|Default|GetStaticMesh) (Math|Vector|Lerp(Vector) "0, 0, 0" (Variables|Default|GetEndPoint) _movement) false false))
        (:Finished
          (Utilities|FlowControl|Delay (Variables|Default|GetDelayDuration))
          (goto _label))))
    (:B
      (Timeline|Movement Reverse))))

(event EventTick
  (params (DeltaSeconds :type Float%20%28single-precision%29))
  (bind _player (Variables|Default|GetPlayer))
  (bind _player_2 (Variables|Default|GetPlayer))
  (bind _player_3 (Variables|Default|GetPlayer))
  (if (Variables|Default|GetIsHolding?)
    (if (Variables|/Game/_Game/MagnetMechanics/BP_Magnet.BP_Magnet_C|GetIsBlackUp? _player_3)
      ;[0.15 0.15 0.15 0.5] Hold
      (CallFunction|TurnOffCollisions)
      (Variables|/Game/_Game/MagnetMechanics/BP_Magnet.BP_Magnet_C|SetCanHorizontalTurn _player_2 false)
      (Variables|/Game/_Game/MagnetMechanics/BP_Magnet.BP_Magnet_C|SetCanMove? _player_2 false)
      (bind _snapplayer (Timeline|SnapPlayerTimeline Play)
        (:Update
          (bind _output_get (Variables|Default|SetSnapTimeline _snapplayer))
          (Transformation|SetActorLocationAndRotation _player (Math|Vector|Lerp(Vector) (Transformation|GetActorLocation _player) (Transformation|GetWorldLocation (Variables|Default|GetBoxCollision)) _output_get))))
      (else
        ;[0.15 0.15 0.15 0.5] Release
        (Physics|Components|PhysicsHandle|ReleaseComponent (Variables|Default|GetPhysicsHandle))
        (CallFunction|TurnonCollision)
        (Variables|/Game/_Game/MagnetMechanics/BP_Magnet.BP_Magnet_C|SetCanHorizontalTurn _player_3 true)
        (Variables|/Game/_Game/MagnetMechanics/BP_Magnet.BP_Magnet_C|SetCanMove? _player_3 true)
        (Default|RedForwardTurnVertically _player_3)
        (Components|Activation|SetActive (Variables|Default|GetBoxCollision) false false)
        (Variables|Default|SetIsHolding? false)
        (Variables|Default|SetIsReleased? true)
        (Utilities|FlowControl|Delay 1.0)
        (Components|Activation|SetActive (Variables|Default|GetBoxCollision) true false)))
    (elif (not (Variables|Default|GetIsReleased?))
      (Physics|Components|PhysicsHandle|ReleaseComponent (Variables|Default|GetPhysicsHandle))
      (Variables|Default|SetIsReleased? true))))

(fn ConstructionScript)