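; Actor component for black magnets that detects objects inside the owner's magnetic radius and signals them to be attracted.
; A looping timer started on BeginPlay periodically runs a stationary single-hit sphere trace at the owner's location on a dedicated trace channel.
; A hit actor implementing BPI_BlackMagneticField becomes TargetActor and receives BlackAttrackMessage; otherwise the target is cleared.
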(event Custom|UpdateBlackMagneticField
  (CallFunction|GetBlackMagneticField))

(event EventBeginPlay
  (Utilities|Time|SetTimerbyEvent (delegate Custom|UpdateBlackMagneticField) 0.2 true))

(fn GetBlackMagneticField
  (bind _returnvalue (Components|GetOwner))
  (bind _returnvalue_2 (Transformation|GetActorLocation _returnvalue))
  (bind (_outhit _returnvalue_3) (Collision|SphereTraceByChannel _returnvalue_2 _returnvalue_2 (Variables|Default|GetBlackMagneticRadius) "TraceTypeQuery5" false 0 "None"))
  (if _returnvalue_3
    (if (Utilities|DoesObjectImplementInterface (.HitActor (Collision|BreakHitResult _outhit)) "/Game/_Game/MagnetMechanics/Magnets/BPI_BlackMagneticField.BPI_BlackMagneticField_C")
      (bind _output_get (Variables|Default|SetTargetActor (.HitActor (Collision|BreakHitResult _outhit))))
      (Class|BPIBlackMagneticField|BlackAttrack(Message) _output_get)
      (else
        (Variables|Default|SetTargetActor 0)))
    (else
      (Variables|Default|SetTargetActor 0))))