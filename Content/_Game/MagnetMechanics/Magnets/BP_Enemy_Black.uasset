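; Black magnetic enemy that homes in on the player and explodes after being pushed or hitting them.
; BlackAttrack arms it and swaps to an attack material if the player's BP_Magnet has an active black magnet component.
; While armed, Tick drives two timelines feeding MoveComponentTo toward the player's Red component.
; StartExplosion and StartEarlyExplosion deactivate it, then use separate delays before the Niagara blast and destruction.
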(event Custom|StartExplosion
  ;[0.15 0.15 0.15 0.5] Explode After Being Pushed
  (Variables|Default|SetIsActivated? false)
  (Variables|Default|SetisPushed? true)
  (Rendering|Material|SetMaterial (Variables|Default|GetCube) 0 "/Game/_Game/Materials/MI_DeactivatedBlack.MI_DeactivatedBlack")
  (Utilities|FlowControl|Delay (Variables|Default|GetExplostionDelay))
  (Components|Activation|SetActive (Variables|Default|GetExplosionNia) true false)
  (Utilities|FlowControl|Delay (Variables|Default|GetDestroyDelay))
  (Actor|DestroyActor))

(event Custom|StartEarlyExplosion
  ;[0.15 0.15 0.15 0.5] Explode when Hit Player
  (Variables|Default|SetIsActivated? false)
  (Variables|Default|SetisPushed? true)
  (Rendering|Material|SetMaterial (Variables|Default|GetCube) 0 "/Game/_Game/Materials/MI_DeactivatedBlack.MI_DeactivatedBlack")
  (Utilities|FlowControl|Delay (Variables|Default|GetXplodEarly))
  (Components|Activation|SetActive (Variables|Default|GetExplosionNia) true false)
  (Utilities|FlowControl|Delay (Variables|Default|GetDestroyDelay))
  (Actor|DestroyActor))

(event EventTick
  (params (DeltaSeconds :type Float%20%28single-precision%29))
  (bind _targetobj (Variables|Default|GetTargetObj))
  (bind _defaultsceneroot (Variables|Default|GetDefaultSceneRoot))
  (bind _red (Variables|/Game/_Game/MagnetMechanics/BP_Magnet.BP_Magnet_C|GetRed _targetobj))
  (if (Variables|Default|GetIsActivated?)
    (if (Variables|Default|GetisPushed?)
      (CallFunction|StartExplosion)
      (else
        ;[0.15 0.15 0.15 0.5] Moving Toward Player
        (Collision|SetCollisionEnabled (Variables|Default|GetCube) "QueryAndPhysics")
        (Utilities|IsValid _red
          (:Is%20Valid
            (bind _enemymove (Timeline|EnemyMove Play)
              (:Update
                (bind _turnlerp (Timeline|TurnLerp Play)
                  (:Update
                    (Components|MoveComponentTo _defaultsceneroot (Math|Vector|Lerp(Vector) (Transformation|GetWorldLocation (Variables|Default|GetDefaultSceneRoot)) (Transformation|GetWorldLocation _red) _enemymove) (Math|Rotator|Lerp(Rotator) (Transformation|GetWorldRotation _defaultsceneroot) (Transformation|GetWorldRotation _red) _turnlerp) false false 0.3 false)))))))))))

(event EventBlackAttrack
  ;[0.15 0.15 0.15 0.5] Detecting Player In Range
  (bind _asbp_magnet (Utilities|Casting|CastToBP_Magnet (Game|GetPlayerCharacter 0)))
  (Utilities|IsValid _asbp_magnet
    (:Is%20Valid
      (bind _output_get (Variables|Default|SetTargetObj _asbp_magnet))
      (Utilities|IsValid (Variables|/Game/_Game/MagnetMechanics/BP_Magnet.BP_Magnet_C|GetBPC_BlackMagnet _output_get)
        (:Is%20Valid
          (if (Components|Activation|IsActive (Variables|/Game/_Game/MagnetMechanics/BP_Magnet.BP_Magnet_C|GetBPC_BlackMagnet _output_get))
            (Rendering|Material|SetMaterial (Variables|Default|GetCube) 0 "/Game/_Game/Materials/MI_ExplosionBlack_Attack.MI_ExplosionBlack_Attack")
            (Variables|Default|SetIsActivated? true)))))))

(event EventBeginPlay
  ;[0.15 0.15 0.15 0.5] Initiate
  (Variables|Default|SetisPushed? false)
  (Variables|Default|SetIsActivated? false)
  (Components|Activation|SetActive (Variables|Default|GetFireNia) true false)
  (Components|Activation|SetActive (Variables|Default|GetExplosionNia) false false))

(fn ConstructionScript)