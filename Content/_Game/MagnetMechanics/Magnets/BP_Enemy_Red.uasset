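; Red magnet enemy that chases the player and self-destructs in an explosion.
; RedAttack activates it if the player BP_Magnet's red magnet component is active, swapping to an explosive material.
; While activated, Tick uses two timelines and MoveComponentTo to pull it toward the player's Black component, or starts the explosion once pushed.
; Separate pushed and player-hit events deactivate it, then run delayed Niagara explosion and destruction.
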(event Custom|StartExplosion
  ;[0.15 0.15 0.15 0.5] Explode After being Pushed
  (Variables|Default|SetIsActivated? false)
  (Variables|Default|SetisPushed? true)
  (Rendering|Material|SetMaterial (Variables|Default|GetCube) 0 "/Game/_Game/Materials/M_DeactivatedRed.M_DeactivatedRed")
  (Utilities|FlowControl|Delay (Variables|Default|GetExplosionDelay))
  (Components|Activation|SetActive (Variables|Default|GetExplosionNia) true false)
  (Utilities|FlowControl|Delay (Variables|Default|GetDestroyDelay))
  (Actor|DestroyActor))

(event Custom|StartEarlyExplosion
  ;[0.15 0.15 0.15 0.5] Explode After Hitting Player
  (Variables|Default|SetIsActivated? false)
  (Variables|Default|SetisPushed? true)
  (Rendering|Material|SetMaterial (Variables|Default|GetCube) 0 "/Game/_Game/Materials/M_DeactivatedRed.M_DeactivatedRed")
  (Utilities|FlowControl|Delay (Variables|Default|GetExplosionEarlyDelay))
  (Components|Activation|SetActive (Variables|Default|GetExplosionNia) true false)
  (Utilities|FlowControl|Delay (Variables|Default|GetDestroyDelay))
  (Actor|DestroyActor))

(event EventTick
  (params (DeltaSeconds :type Float%20%28single-precision%29))
  (bind _targetobj (Variables|Default|GetTargetObj))
  (bind _defaultsceneroot (Variables|Default|GetDefaultSceneRoot))
  (bind _black (Variables|/Game/_Game/MagnetMechanics/BP_Magnet.BP_Magnet_C|GetBlack _targetobj))
  (if (Variables|Default|GetIsActivated?)
    (if (Variables|Default|GetisPushed?)
      (CallFunction|StartExplosion)
      (else
        ;[0.15 0.15 0.15 0.5] Moving Toward Player
        (Collision|SetCollisionEnabled (Variables|Default|GetCube) "QueryAndPhysics")
        (Utilities|IsValid _black
          (:Is%20Valid
            (bind _enemymove (Timeline|EnemyMove Play)
              (:Update
                (bind _turnlerp (Timeline|TurnLerp Play)
                  (:Update
                    (Components|MoveComponentTo _defaultsceneroot (Math|Vector|Lerp(Vector) (Transformation|GetWorldLocation (Variables|Default|GetDefaultSceneRoot)) (Transformation|GetWorldLocation _black) _enemymove) (Math|Rotator|Lerp(Rotator) (Transformation|GetWorldRotation _defaultsceneroot) (Transformation|GetWorldRotation _black) _turnlerp) false false 0.3 false)))))))))))

(event EventRedAttrack
  ;[0.15 0.15 0.15 0.5] Detecting Player In Range
  (if (not (Variables|Default|GetIsActivated?))
    (bind _asbp_magnet (Utilities|Casting|CastToBP_Magnet (Game|GetPlayerCharacter 0)))
    (Utilities|IsValid _asbp_magnet
      (:Is%20Valid
        (bind _output_get (Variables|Default|SetTargetObj _asbp_magnet))
        (Utilities|IsValid (Variables|/Game/_Game/MagnetMechanics/BP_Magnet.BP_Magnet_C|GetBPC_RedMagnet _output_get)
          (:Is%20Valid
            (if (Components|Activation|IsActive (Variables|/Game/_Game/MagnetMechanics/BP_Magnet.BP_Magnet_C|GetBPC_RedMagnet _output_get))
              (Rendering|Material|SetMaterial (Variables|Default|GetCube) 0 "/Game/_Game/Materials/MI_ExplosionRed.MI_ExplosionRed")
              (Variables|Default|SetIsActivated? true))))))))

(event EventBeginPlay
  ;[0.15 0.15 0.15 0.5] Initiate
  (Components|Activation|SetActive (Variables|Default|GetFireNiagara) true false)
  (Components|Activation|SetActive (Variables|Default|GetExplosionNia) false false))

(fn ConstructionScript)