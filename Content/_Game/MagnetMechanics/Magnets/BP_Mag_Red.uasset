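; BP_Mag_Red is a red magnetic pickup, with a Tin component, that the player's active red magnet pulls in and carries.
; RedAttrack checks and updates BP_Magnet's collection state, moves the root to RedDestCol, then starts a looping timer that keeps it following via MagIsActivated.
; Release resets the player's flags, zeroes Tin's velocity, invalidates the timer and destroys the actor after a delay.
; The Compressor drop-off logic is disconnected from its empty overlap event.
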(event OnComponentBeginOverlap(Collision)
  (params (OverlappedComponent :type Primitive%20Component%20Object%20Reference) (OtherActor :type Actor%20Object%20Reference) (OtherComp :type Primitive%20Component%20Object%20Reference) (OtherBodyIndex :type Integer) (bFromSweep :type Boolean) (SweepResult :type Hit%20Result%20Structure%20%28by%20ref%29))
  ;[0.15 0.15 0.15 0.5] Broken
)

(event Custom|MagIsActivated
  (bind _target (Variables|Components|GetTarget))
  (if (not (Variables|Default|GetisRealsing?))
    (Collision|SetCollisionEnabled (Variables|Components|GetTin) "NoCollision")
    (Components|MoveComponentTo (Variables|Components|GetDefaultSceneRoot) (Transformation|GetWorldLocation _target) (Transformation|GetWorldRotation _target) false false 0.2 false)))

(event Custom|Release
  (bind _playerbp (Variables|Default|GetPlayerBP))
  (Variables|Default|SetisRealsing? true)
  (Variables|/Game/_Game/MagnetMechanics/BP_Magnet.BP_Magnet_C|SetisRedCollected? _playerbp false)
  (Variables|/Game/_Game/MagnetMechanics/BP_Magnet.BP_Magnet_C|SetIsRedFull? _playerbp false)
  (Variables|/Game/_Game/MagnetMechanics/BP_Magnet.BP_Magnet_C|SetCanVertTurn? _playerbp true)
  (Physics|SetPhysicsLinearVelocity (Variables|Components|GetTin) "0, 0, 0" false "None")
  (Collision|SetCollisionEnabled (Variables|Components|GetTin) "QueryOnly")
  (Utilities|Time|InvalidateTimerHandle (Variables|Default|GetTimerHandle))
  (Utilities|FlowControl|Delay 0.5)
  (Actor|DestroyActor))

(event EventRedAttrack
  (bind _asbp_magnet (Utilities|Casting|CastToBP_Magnet (Game|GetPlayerCharacter 0)))
  (Utilities|IsValid (Actor|GetComponentbyClass _asbp_magnet "/Game/_Game/MagnetMechanics/Magnets/BPC_RedMagnet.BPC_RedMagnet_C")
    (:Is%20Valid
      (if (Components|Activation|IsActive (Actor|GetComponentbyClass _asbp_magnet "/Game/_Game/MagnetMechanics/Magnets/BPC_RedMagnet.BPC_RedMagnet_C"))
        (bind _output_get (Variables|Default|SetPlayerBP _asbp_magnet))
        (if (not (Variables|/Game/_Game/MagnetMechanics/BP_Magnet.BP_Magnet_C|GetisRedCollected? _output_get))
          (if (Variables|/Game/_Game/MagnetMechanics/BP_Magnet.BP_Magnet_C|GetCanCollect? (Variables|Default|GetPlayerBP))
            (Variables|/Game/_Game/MagnetMechanics/BP_Magnet.BP_Magnet_C|SetCanVertTurn? (Variables|Default|GetPlayerBP) false)
            (Variables|/Game/_Game/MagnetMechanics/BP_Magnet.BP_Magnet_C|SetisRedCollected? (Variables|Default|GetPlayerBP) true)
            (Utilities|IsValid (Variables|/Game/_Game/MagnetMechanics/BP_Magnet.BP_Magnet_C|GetRedDestCol (Variables|Default|GetPlayerBP))
              (:Is%20Valid
                (Variables|Components|SetTarget (Variables|/Game/_Game/MagnetMechanics/BP_Magnet.BP_Magnet_C|GetRedDestCol (Variables|Default|GetPlayerBP)))
                (Collision|SetCollisionEnabled (Variables|Components|GetTin) "QueryOnly")
                (Components|MoveComponentTo (Variables|Components|GetDefaultSceneRoot) (Transformation|GetWorldLocation (Variables|Components|GetTarget)) (Transformation|GetWorldRotation (Variables|Components|GetTarget)) false false 0.5 false)
                (if (not (Variables|Default|GetisRealsing?))
                  (bind _returnvalue (Utilities|Time|SetTimerbyEvent (delegate Custom|MagIsActivated) (Variables|Default|GetAttrackFrequency) true))
                  (Variables|Default|SetTimerHandle _returnvalue))))))))))

(fn ConstructionScript)