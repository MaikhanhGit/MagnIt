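; Black magnet object with a physics-simulated cube that gets pulled toward the player's magnet.
; BlackAttrack activates it when the player character, a BP_Magnet, has an active BPCBlackMagnet component.
; While activated, Tick swaps to the deactivated material if the player's IsBlackPushed is set.
; Otherwise it enables collision and uses nested timelines with MoveComponentTo to lerp the root toward the player's Red target's location and rotation.
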(event EventTick
  (params (DeltaSeconds :type Float%20%28single-precision%29))
  (bind _targetobj (Variables|Default|GetTargetObj))
  (bind _defaultsceneroot (Variables|Default|GetDefaultSceneRoot))
  (bind _red (Variables|/Game/_Game/MagnetMechanics/BP_Magnet.BP_Magnet_C|GetRed _targetobj))
  (if (Variables|Default|GetIsActivated?)
    (if (Variables|/Game/_Game/MagnetMechanics/BP_Magnet.BP_Magnet_C|GetIsBlackPushed? (Variables|Default|GetTargetObj))
      (Rendering|Material|SetMaterial (Variables|Default|GetCube) 0 "/Game/_Game/Materials/MI_DeactivatedBlack.MI_DeactivatedBlack")
      (else
        (Collision|SetCollisionEnabled (Variables|Default|GetCube) "QueryAndPhysics")
        (Utilities|IsValid _red
          (:Is%20Valid
            (bind _enemymove (Timeline|EnemyMove Play)
              (:Update
                (bind _turnlerp (Timeline|TurnLerp Play)
                  (:Update
                    (Components|MoveComponentTo _defaultsceneroot (Math|Vector|Lerp(Vector) (Transformation|GetWorldLocation (Variables|Default|GetDefaultSceneRoot)) (Transformation|GetWorldLocation _red) _enemymove) (Math|Rotator|Lerp(Rotator) (Transformation|GetWorldRotation _defaultsceneroot) (Transformation|GetWorldRotation _red) _turnlerp) false false 0.3 false)))))))))))

(event EventBlackAttrack
  (bind _asbp_magnet (Utilities|Casting|CastToBP_Magnet (Game|GetPlayerCharacter 0)))
  (Utilities|IsValid _asbp_magnet
    (:Is%20Valid
      (bind _output_get (Variables|Default|SetTargetObj _asbp_magnet))
      (Utilities|IsValid (Variables|/Game/_Game/MagnetMechanics/BP_Magnet.BP_Magnet_C|GetBPC_BlackMagnet _output_get)
        (:Is%20Valid
          (if (Components|Activation|IsActive (Variables|/Game/_Game/MagnetMechanics/BP_Magnet.BP_Magnet_C|GetBPC_BlackMagnet _output_get))
            (Variables|Default|SetIsActivated? true)))))))

(event EventBeginPlay
  (Variables|Default|SetisPushed? false)
  (Variables|Default|SetIsActivated? false)
  (Physics|SetSimulatePhysics (Variables|Default|GetCube) true))

(fn ConstructionScript)