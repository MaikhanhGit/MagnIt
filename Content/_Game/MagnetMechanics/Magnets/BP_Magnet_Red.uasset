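; BP_Magnet_Red is a red magnet object that the player's BP_Magnet character can activate.
; RedAttrack sets IsActivated when the player's red magnet component is active.
; Tick applies a deactivated red material once the object is both activated and pushed, though IsPushed is only ever cleared here.
; A disconnected timeline chain for pulling it toward the player's Black component never runs.
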(event EventTick
  (params (DeltaSeconds :type Float%20%28single-precision%29))
  (if (Variables|Default|GetIsActivated?)
    (if (Variables|Default|GetisPushed?)
      (Rendering|Material|SetMaterial (Variables|Default|GetCube) 0 "/Game/_Game/Materials/M_DeactivatedRed.M_DeactivatedRed"))))

(event EventRedAttrack
  (if (not (Variables|Default|GetIsActivated?))
    (bind _asbp_magnet (Utilities|Casting|CastToBP_Magnet (Game|GetPlayerCharacter 0)))
    (Utilities|IsValid _asbp_magnet
      (:Is%20Valid
        (bind _output_get (Variables|Default|SetTargetObj _asbp_magnet))
        (Utilities|IsValid (Variables|/Game/_Game/MagnetMechanics/BP_Magnet.BP_Magnet_C|GetBPC_RedMagnet _output_get)
          (:Is%20Valid
            (if (Components|Activation|IsActive (Variables|/Game/_Game/MagnetMechanics/BP_Magnet.BP_Magnet_C|GetBPC_RedMagnet _output_get))
              (Variables|Default|SetIsActivated? true))))))))

(event EventBeginPlay
  (Variables|Default|SetisPushed? false)
  (Variables|Default|SetIsActivated? false))

(fn ConstructionScript)