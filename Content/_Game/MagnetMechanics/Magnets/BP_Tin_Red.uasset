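; BP_Tin_Red is a red tin that the player's BP_Magnet pulls in while its red magnet component is active.
; RedAttrack claims the player's single red slot, disables tin physics and moves it to RedDestCol.
; A looping timer repeatedly re-targets that destination with collision off, keeping the tin following it.
; Release stops the timer and velocity, then activates Niagara particles after a short delay and destroys the actor.
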(event Custom|MagIsActivated
  (bind _target (Variables|Components|GetTarget))
  ;[0.15 0.15 0.15 0.5] Magnetic Attraction
  (if (not (Variables|Default|GetisReleasing?))
    (Collision|SetCollisionEnabled (Variables|Components|GetTin) "NoCollision")
    (Components|MoveComponentTo (Variables|Components|GetDefaultSceneRoot) (Transformation|GetWorldLocation _target) (Transformation|GetWorldRotation _target) false false 0.2 false)))

(event Custom|Release
  ;[0.15 0.15 0.15 0.5] Realease
  (Variables|Default|SetisReleasing? true)
  (Physics|SetPhysicsLinearVelocity (Variables|Components|GetTin) "0, 0, 0" false "None")
  (Collision|SetCollisionEnabled (Variables|Components|GetTin) "QueryOnly")
  (Utilities|Time|InvalidateTimerHandle (Variables|Default|GetTimerHandle))
  (Utilities|FlowControl|Delay 0.3)
  (Components|Activation|SetActive (Variables|Default|GetNS_PlayerParticles2) true false)
  (Utilities|FlowControl|Delay 0.5)
  (Actor|DestroyActor))

(event EventBeginPlay
  (Components|Activation|SetActive (Variables|Default|GetNS_PlayerParticles2) false false))

(event EventRedAttrack
  ;[0.15 0.15 0.15 0.5] Magnetic Attraction
  (if (not (Variables|Default|GetisReleasing?))
    (bind _asbp_magnet (Utilities|Casting|CastToBP_Magnet (Game|GetPlayerCharacter 0)))
    (Utilities|IsValid (Actor|GetComponentbyClass _asbp_magnet "/Game/_Game/MagnetMechanics/Magnets/BPC_RedMagnet.BPC_RedMagnet_C")
      (:Is%20Valid
        (if (Components|Activation|IsActive (Actor|GetComponentbyClass _asbp_magnet "/Game/_Game/MagnetMechanics/Magnets/BPC_RedMagnet.BPC_RedMagnet_C"))
          (bind _output_get (Variables|Default|SetPlayerBP _asbp_magnet))
          (if (not (Variables|/Game/_Game/MagnetMechanics/BP_Magnet.BP_Magnet_C|GetisRedCollected? _output_get))
            (Utilities|IsValid (Variables|/Game/_Game/MagnetMechanics/BP_Magnet.BP_Magnet_C|GetRedDestCol (Variables|Default|GetPlayerBP))
              (:Is%20Valid
                (Variables|Components|SetTarget (Variables|/Game/_Game/MagnetMechanics/BP_Magnet.BP_Magnet_C|GetRedDestCol (Variables|Default|GetPlayerBP)))
                (Variables|/Game/_Game/MagnetMechanics/BP_Magnet.BP_Magnet_C|SetisRedCollected? (Variables|Default|GetPlayerBP) true)
                (Physics|SetSimulatePhysics (Variables|Components|GetTin) false)
                (Collision|SetCollisionEnabled (Variables|Components|GetTin) "QueryOnly")
                (Components|MoveComponentTo (Variables|Components|GetDefaultSceneRoot) (Transformation|GetWorldLocation (Variables|Components|GetTarget)) (Transformation|GetWorldRotation (Variables|Components|GetTarget)) false false 0.5 false)
                (if (Variables|Default|GetisReleasing?)
                  (if (Class|KismetSystemLibrary|TimerExistsHandle (Variables|Default|GetTimerHandle))
                    (Utilities|Time|InvalidateTimerHandle (Variables|Default|GetTimerHandle)))
                  (else
                    (bind _returnvalue (Utilities|Time|SetTimerbyEvent (delegate Custom|MagIsActivated) (Variables|Default|GetAttrackFrequency) true))
                    (Variables|Default|SetTimerHandle _returnvalue))))
              (:Is%20Not%20Valid
                (Variables|/Game/_Game/MagnetMechanics/BP_Magnet.BP_Magnet_C|SetisRedCollected? (Variables|Default|GetPlayerBP) false)))))))))

(fn ConstructionScript)