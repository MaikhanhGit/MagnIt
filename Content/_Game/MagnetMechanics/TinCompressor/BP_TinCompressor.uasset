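; Tin compressor in the magnet mechanics that makes BP_Magnet release its collected red and black tins.
; When a PlayerKillCollision component enters the capsule, it calls the magnet's release function for each held tin and records collected/released flags.
; Overlapping actors without the Player tag are destroyed.
; BeginPlay caches the release location; the tin-movement and reset logic is disconnected and never runs.
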(event OnComponentBeginOverlap(Capsule)
  (params (OverlappedComponent :type Primitive%20Component%20Object%20Reference) (OtherActor :type Actor%20Object%20Reference) (OtherComp :type Primitive%20Component%20Object%20Reference) (OtherBodyIndex :type Integer) (bFromSweep :type Boolean) (SweepResult :type Hit%20Result%20Structure%20%28by%20ref%29))
  (Utilities|FlowControl|Sequence
    (:then_0
      (if (Components|ComponentHasTag OtherComp "PlayerKillCollision")
        (bind _asbp_magnet (Utilities|Casting|CastToBP_Magnet OtherActor))
        (Utilities|IsValid _asbp_magnet
          (:Is%20Valid
            (Variables|Default|SetPlayerRef _asbp_magnet)
            (Utilities|FlowControl|Sequence
              (:then_0
                ;[0.15 0.15 0.15 0.5] Check For Red Tin
                (if (Variables|/Game/_Game/MagnetMechanics/BP_Magnet.BP_Magnet_C|GetisRedCollected? (Variables|Default|GetPlayerRef))
                  (Utilities|IsValid (Variables|/Game/_Game/MagnetMechanics/BP_Magnet.BP_Magnet_C|GetCollectedRedTin (Variables|Default|GetPlayerRef))
                    (:Is%20Valid
                      (Variables|Default|SetisRedCollected? true)
                      (Default|ReleaseRedTin (Variables|Default|GetPlayerRef))
                      (Variables|Default|SetisRedReleased? true))
                    (:Is%20Not%20Valid
                      (Variables|Default|SetisRedCollected? false)))))
              (:then_1
                ;[0.15 0.15 0.15 0.5] Check for Black Tin
                (if (Variables|/Game/_Game/MagnetMechanics/BP_Magnet.BP_Magnet_C|GetisBlackCollected? (Variables|Default|GetPlayerRef))
                  (Utilities|IsValid (Variables|/Game/_Game/MagnetMechanics/BP_Magnet.BP_Magnet_C|GetCollectedBlackTin (Variables|Default|GetPlayerRef))
                    (:Is%20Valid
                      (Variables|Default|SetisBlackCollected? true)
                      (Default|ReleaseBlackTin (Variables|Default|GetPlayerRef))
                      (Variables|Default|SetisBlackReleased true))
                    (:Is%20Not%20Valid
                      (Variables|Default|SetisBlackCollected? false))))))))))
    (:then_1
      (if (not (Actor|ActorHasTag OtherActor "Player"))
        (Actor|DestroyActor OtherActor)))))

(event EventBeginPlay
  (Variables|Default|SetTinReleaseLocation (Transformation|GetWorldLocation (Variables|Default|GetLocation))))

(fn ConstructionScript)